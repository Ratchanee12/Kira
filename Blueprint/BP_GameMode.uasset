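; Game mode that saves and restores the player character's transform through a single save slot.
; On BeginPlay it loads the slot and moves the ThirdPersonCharacter to the stored transform, or creates an empty BP_SaveGame if none exists.
; SaveGame writes the current transform into that slot.
; LoadGame just restarts the level so BeginPlay reapplies the save, while RestartLevel deletes the save before restarting.
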(event Custom|SaveGame
  ;[1 1 1] SaveGame
  (bind _returnvalue (SaveGame|LoadGamefromSlot "save1"))
  (bind _asbp_save_game (Utilities|Casting|CastToBP_SaveGame _returnvalue))
  (Variables|/Game/Kira/Blueprint/BP_SaveGame.BP_SaveGame_C|SetTransform _asbp_save_game (Transformation|GetActorTransform (.AsThird%20Person%20Character (Utilities|Casting|CastToThirdPersonCharacter (Game|GetPlayerCharacter 0)))))
  (SaveGame|SaveGametoSlot _asbp_save_game "save1"))

(event Custom|LoadGame
  ;[1 1 1] LoadGame
  (Development|ExecuteConsoleCommand "RestartLevel" 0))

(event Custom|RestartLevel
  ;[1 1 1] Delete Save + Restart
  (SaveGame|DeleteGameinSlot "save1")
  (Development|ExecuteConsoleCommand "RestartLevel" 0))

(event EventBeginPlay
  (bind _returnvalue (SaveGame|DoesSaveGameExist "save1"))
  (if _returnvalue
    ;[1 1 1] Load Game Funtion
    (bind _returnvalue_2 (SaveGame|LoadGamefromSlot "save1"))
    (bind _asbp_save_game (Utilities|Casting|CastToBP_SaveGame _returnvalue_2))
    (bind _asthird_person_character (Utilities|Casting|CastToThirdPersonCharacter (Game|GetPlayerCharacter 0)))
    (Transformation|SetWorldTransform (Variables|/Script/Engine.Actor|GetRootComponent _asthird_person_character) (Variables|/Game/Kira/Blueprint/BP_SaveGame.BP_SaveGame_C|GetTransform _asbp_save_game) false false)
    (else
      ;[1 1 1] Create Save File
      (bind _returnvalue_3 (SaveGame|CreateSaveGameObject "/Game/Kira/Blueprint/BP_SaveGame.BP_SaveGame_C"))
      (SaveGame|SaveGametoSlot _returnvalue_3 "save1"))))

(event EventTick
  (params (DeltaSeconds :type Float%20%28single-precision%29)))

(fn ConstructionScript)